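; BP_MenuCharacter is the main menu's character, which adds the default input mapping and plays menu music when it begins play.
; Each tick it moves along world X at Speed and derives Score from the distance travelled.
; MenuToGame shows a fading loading widget, waits a random few seconds, then opens the MainGamePlay level.
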(event Custom|MenuToGame
  (bind _returnvalue (UserInterface|CreateWidget "/Game/Blueprints/Widgets/WBP_Loading.WBP_Loading_C"))
  (bind _output_get (Variables|Default|SetLoading _returnvalue))
  (UserInterface|Viewport|AddtoViewport _output_get 0)
  (UserInterface|Animation|PlayAnimation _output_get (Variables|/Game/Blueprints/Widgets/WBP_Loading.WBP_Loading_C|GetLoadingFade (Variables|Default|GetLoading)) 0.0 1 "Forward" 1.0 false)
  (Utilities|FlowControl|Delay (Math|Random|RandomFloatinRange 5.5 7.5))
  (Game|OpenLevel(byName) "MainGamePlay"))

(event EventBeginPlay
  (bind _asplayer_controller (Utilities|Casting|CastToPlayerController (Pawn|GetController)))
  (Utilities|IsValid (PlayerController|LocalPlayerSubsystems|GetEnhancedInputLocalPlayerSubsystem _asplayer_controller)
    (:Is%20Valid
      (Input|AddMappingContext (PlayerController|LocalPlayerSubsystems|GetEnhancedInputLocalPlayerSubsystem _asplayer_controller) "/Game/ThirdPerson/Input/IMC_Default.IMC_Default" 0 "(bIgnoreAllPressedKeysUntilRelease=True,bForceImmediately=False,bNotifyUserSettings=False)")
      (Audio|PlaySound2D "/Game/Assets/Sounds/Musics/Menu_Cue.Menu_Cue" 1.0 1.0 0.0 0 0))))

(event EventTick
  (params (DeltaSeconds :type Float%20%28single-precision%29))
  (bind _returnvalue (Transformation|GetActorLocation))
  (bind (_x _y _z) (Math|Vector|BreakVector _returnvalue))
  (Variables|Default|SetDelta%20Seconds DeltaSeconds)
  (Transformation|SetActorLocation (Math|Vector|MakeVector (+ (.X (Math|Vector|BreakVector (Transformation|GetActorLocation))) (* (Variables|Default|GetSpeed) (Variables|Default|GetDelta%20Seconds))) _y _z) false false)
  (Variables|Default|SetScore (Math|Float|Truncate (/ (.x (Transformation|GetActorLocation)) 1e+02))))

(fn ConstructionScript)