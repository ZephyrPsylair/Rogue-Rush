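; BP_Spawner generates an endless track of random platforms along the X axis for the runner character.
; BeginPlay lays an initial row of half-scale platforms picked from PlatformClass, advancing SpawnLocation by PlatformLength each time.
; Tick appends another when the player nears the end, resetting a looping CheckAndDestroy timer.
; That function destroys platforms beyond DespawnThreshold behind the player, removing index 0 while iterating SpawnedPlatforms.
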(event EventBeginPlay
  (bind _asbp_runner_character (Utilities|Casting|CastToBP_RunnerCharacter (Game|GetPlayerCharacter 0)))
  (Variables|Default|SetPlayer _asbp_runner_character)
  (for _index (range 0 5)
    (bind _returnvalue (Game|SpawnActorfromClass (Utilities|Array|Get(acopy) (Variables|Default|GetPlatformClass) (Math|Random|RandomIntegerinRange 0 24)) (Math|Transform|MakeTransform (Variables|Default|GetSpawnLocation) "0, 0, 0" "0.500000,0.500000,0.500000") "Undefined" "MultiplyWithRoot" 0 0))
    (Utilities|Array|Add (Variables|Default|GetSpawnedPlatforms) _returnvalue)
    (Variables|Default|SetSpawnLocation (Math|Vector|MakeVector (+ (.x (Variables|Default|GetSpawnLocation)) (Variables|Default|GetPlatformLength)) (.y (Variables|Default|GetSpawnLocation)) (.z (Variables|Default|GetSpawnLocation))))))

(event EventTick
  (params (DeltaSeconds :type Float%20%28single-precision%29))
  (if (> (+ (.x (Transformation|GetActorLocation (Variables|Default|GetPlayer))) (Variables|Default|GetSpawnThreshold)) (.x (Variables|Default|GetSpawnLocation)))
    (bind _returnvalue (Game|SpawnActorfromClass (Utilities|Array|Get(acopy) (Variables|Default|GetPlatformClass) (Math|Random|RandomIntegerinRange 0 24)) (Math|Transform|MakeTransform (Variables|Default|GetSpawnLocation) "0, 0, 0" "0.500000,0.500000,0.500000") "Undefined" "MultiplyWithRoot" 0 0))
    (Utilities|Array|Add (Variables|Default|GetSpawnedPlatforms) _returnvalue)
    (Variables|Default|SetSpawnLocation (Math|Vector|MakeVector (+ (.x (Variables|Default|GetSpawnLocation)) (Variables|Default|GetPlatformLength)) (.y (Variables|Default|GetSpawnLocation)) (.z (Variables|Default|GetSpawnLocation))))
    (Utilities|Time|SetTimerbyFunctionName 0 "CheckAndDestroy" 0.5 true)))

(fn ConstructionScript)

(fn CheckandDestroy
  (for _array_element (Variables|Default|GetSpawnedPlatforms)
    (if (< (.x (Transformation|GetActorLocation _array_element)) (- (.x (Transformation|GetActorLocation (Variables|Default|GetPlayer))) (Variables|Default|GetDespawnThreshold)))
      (Actor|DestroyActor _array_element)
      (Utilities|Array|RemoveIndex (Variables|Default|GetSpawnedPlatforms)))))