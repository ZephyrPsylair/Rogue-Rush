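; BP_RollingCity is a backdrop actor that keeps four city components moving along with the runner character.
; On BeginPlay it caches the player as BP_RunnerCharacter.
; Each Tick it sets every component's relative X to the player's world X at a fixed height below the origin.
; Three layers yaw at different fixed per-frame rates, so their speed depends on frame rate, while the fourth does not spin.
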(event EventBeginPlay
  (bind _asbp_runner_character (Utilities|Casting|CastToBP_RunnerCharacter (Game|GetPlayerCharacter 0)))
  (Variables|Default|SetPlayer _asbp_runner_character))

(event Collision|EventActorBeginOverlap
  (params (OtherActor :type Actor%20Object%20Reference)))

(event EventTick
  (params (DeltaSeconds :type Float%20%28single-precision%29))
  (Variables|Default|SetPlayerLocation (Transformation|GetActorLocation (Variables|Default|GetPlayer)))
  (Transformation|SetRelativeLocationAndRotation (Variables|Default|GetCity1) (Math|Vector|MakeVector (.x (Variables|Default|GetPlayerLocation)) 0.0 -7e+02) (Math|Rotator|MakeRotator 0.0 0.0 (Variables|Default|GetRotation1)) false false)
  (Variables|Default|SetRotation1 (+ (Variables|Default|GetRotation1) 0.02))
  (Transformation|SetRelativeLocationAndRotation (Variables|Default|GetCity2) (Math|Vector|MakeVector (.x (Variables|Default|GetPlayerLocation)) 0.0 -7e+02) (Math|Rotator|MakeRotator 0.0 0.0 (Variables|Default|GetRotation2)) false false)
  (Variables|Default|SetRotation2 (+ (Variables|Default|GetRotation2) 0.01))
  (Transformation|SetRelativeLocationAndRotation (Variables|Default|GetCity3) (Math|Vector|MakeVector (.x (Variables|Default|GetPlayerLocation)) 0.0 -7e+02) (Math|Rotator|MakeRotator 0.0 0.0 (Variables|Default|GetRotation3)) false false)
  (Variables|Default|SetRotation3 (+ (Variables|Default|GetRotation3) 0.009))
  (Transformation|SetRelativeLocationAndRotation (Variables|Default|GetCity4) (Math|Vector|MakeVector (.x (Variables|Default|GetPlayerLocation)) 0.0 -7e+02) "0, 0, 0" false false))

(fn ConstructionScript)